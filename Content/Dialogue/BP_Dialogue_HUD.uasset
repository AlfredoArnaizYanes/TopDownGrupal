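; Dialogue manager actor that creates a hidden dialogue widget on BeginPlay and shows conversations from a data table by row ID.
; Normal rows step through their text lines and hide the widget after the last; Selection rows show a prompt with two responses.
; UpdateIndex moves the widget's highlighted choice, and continuing from a selection opens the row linked to that response, allowing branching.
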(event `self.ReceiveBeginPlay`
  (bind _returnvalue (`|CreateWidget` "/Game/Dialogue/UW_Dialog.UW_Dialog_C" (`GameplayStatics.GetPlayerController` 0)))
  (bind _output_get (set `self.DialogoWidget` _returnvalue))
  (`UserWidget.AddToViewport` _output_get 0)
  (`Widget.SetVisibility` _output_get "Hidden"))

(event `Show Dialogue`
  (params (ID :type Name))
  (`self.ShowDTDialog` ID))

(event `Continue with Dialogue`
  (`self.ContinueWithDialogue`))

(event `Update Index`
  (params (Left :type Boolean))
  (`/Game/Dialogue/UW_Dialog.Update Selection` (`self.DialogoWidget`) Left))

(fn `ContinueWithDialogue`
  (if (`self.ShowingNormalDialog`)
    (bind _returnvalue (`|GetDataTableRow` (`self.DialogoDT`) (`self.CurrentID`))
      (:`then`
        (bind _result (`/Engine/EditorBlueprintResources/StandardMacros.IncrementInt` (`self.DialogIndex`))
          (:`  `
            (bind _text (break `/Game/Dialogue/F_Dialogue` _returnvalue))
            (if (< _result (`KismetArrayLibrary.Array_Length` _text))
              (`/Game/Dialogue/UW_Dialog.Set Normal Dialog` (`self.DialogoWidget`) (`KismetTextLibrary.Conv_StringToText` (`|GetArrayItem` _text _result)))
              (else
                (`Widget.SetVisibility` (`self.DialogoWidget`) "Hidden")
                (set `self.CurrentID` "None")
                (set `self.ShowingNormalDialog` false)))))))
    (elif (`self.ShowingSelection`)
      (bind _returnvalue_2 (`|GetDataTableRow` (`self.DialogoDT`) (`self.CurrentID`))
        (:`then`
          (bind (_output_text _output_id) (break `/Game/Dialogue/F_DialogueResponse` (`|GetArrayItem` (`.Responses_15_46A62CB44BDEA77E94B4128039EBEBCF` (break `/Game/Dialogue/F_Dialogue` _returnvalue_2)) (`/Game/Dialogue/UW_Dialog.SelectionIndex` (`self.DialogoWidget`)))))
          (`self.ShowDTDialog` _output_id))))))

(fn `ShowDTDialog`
  (params (ID :type Name))
  (locals (NewLocalVar :type Name))
  (bind _dialogowidget (`self.DialogoWidget`))
  (bind _returnvalue (`|GetDataTableRow` (`self.DialogoDT`) ID)
    (:`then`
      (bind (_text _type _responses) (break `/Game/Dialogue/F_Dialogue` _returnvalue))
      (switch `/Game/Dialogue/E_DialogueType` _type
        (:`NewEnumerator0`
          (bind _output_get (set `self.DialogIndex` 0))
          (`/Game/Dialogue/UW_Dialog.Set Normal Dialog` (`self.DialogoWidget`) (`KismetTextLibrary.Conv_StringToText` (`|GetArrayItem` _text _output_get)))
          (`Widget.SetVisibility` (`self.DialogoWidget`) "Visible")
          (set `self.ShowingNormalDialog` true)
          (set `self.CurrentID` (`local.ID`)))
        (:`NewEnumerator1`
          (set `self.ShowingSelection` true)
          (bind _output_text (break `/Game/Dialogue/F_DialogueResponse` (`|GetArrayItem` _responses)))
          (bind _output_text_2 (break `/Game/Dialogue/F_DialogueResponse` (`|GetArrayItem` _responses 1)))
          (`/Game/Dialogue/UW_Dialog.Set Selection Dialogue` _dialogowidget (`KismetTextLibrary.Conv_StringToText` (`|GetArrayItem` _text)) (`KismetTextLibrary.Conv_StringToText` _output_text) (`KismetTextLibrary.Conv_StringToText` _output_text_2))
          (`Widget.SetVisibility` _dialogowidget "Visible")
          (set `self.CurrentID` (`local.ID`)))))))

(fn `UserConstructionScript`)